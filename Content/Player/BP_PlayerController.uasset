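; Player controller that sets up the main HUD and provides a save hotkey.
; On BeginPlay, the local controller creates WB_MainHUD, adds it to the viewport and switches input to game-only.
; Pressing L casts the game mode to CGameMode, calls its WriteSaveGame and prints a confirmation.
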(event EventBlueprintBeginPlayingState
  (|CallParentFunction))

(event EventBeginPlay
  (if (Pawn|IsLocalController)
    (bind _returnvalue (UserInterface|CreateWidget "/Game/UI/WB_MainHUD.WB_MainHUD_C"))
    (UserInterface|Viewport|AddtoViewport _returnvalue 0)
    (Input|SetInputModeGameOnly self)))

(event Input|KeyboardEvents|L
  (params (Key :type Key%20Structure :default "None"))
  (:Pressed
    (bind _ascgame_mode (Utilities|Casting|CastToCGameMode (Game|GetGameMode)))
    (Class|CGameMode|WriteSaveGame _ascgame_mode)
    (Development|PrintString "Saved")))

(fn ConstructionScript)